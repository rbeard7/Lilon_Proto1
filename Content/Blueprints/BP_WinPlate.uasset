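; BP_WinPlate is a goal plate for push blocks that shows whether a target block is resting on it.
; On BeginPlay it puts a dynamic instance of the push block material on its plane, glowing red.
; Box overlap events turn it green when the mesh of a BP_PushBlock flagged as Target enters, and red when it leaves.
; It only changes color and triggers no win logic itself.
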(event OnComponentBeginOverlap(Box)
  (params (OverlappedComponent :type Primitive%20Component%20Object%20Reference) (OtherActor :type Actor%20Object%20Reference) (OtherComp :type Primitive%20Component%20Object%20Reference) (OtherBodyIndex :type Integer) (bFromSweep :type Boolean) (SweepResult :type Hit%20Result%20Structure%20%28by%20ref%29))
  (bind _asbp_push_block (Utilities|Casting|CastToBP_PushBlock OtherActor))
  (if (== (Variables|/Game/Blueprints/BP_PushBlock.BP_PushBlock_C|GetStaticMesh _asbp_push_block) OtherComp)
    (if (Variables|/Game/Blueprints/BP_PushBlock.BP_PushBlock_C|GetTarget? _asbp_push_block)
      (Rendering|Material|SetVectorParameterValue (stale EventBeginPlay _returnvalue) "Color" "(R=0.000000,G=1.000000,B=0.000000,A=1.000000)" :!class /Script/Engine.MaterialInstanceDynamic))))

(event OnComponentEndOverlap(Box)
  (params (OverlappedComponent :type Primitive%20Component%20Object%20Reference) (OtherActor :type Actor%20Object%20Reference) (OtherComp :type Primitive%20Component%20Object%20Reference) (OtherBodyIndex :type Integer))
  (bind _asbp_push_block (Utilities|Casting|CastToBP_PushBlock OtherActor))
  (if (== (Variables|/Game/Blueprints/BP_PushBlock.BP_PushBlock_C|GetStaticMesh _asbp_push_block) OtherComp)
    (if (Variables|/Game/Blueprints/BP_PushBlock.BP_PushBlock_C|GetTarget? _asbp_push_block)
      (Rendering|Material|SetVectorParameterValue (stale EventBeginPlay _returnvalue) "Color" "(R=1.000000,G=0.000000,B=0.000000,A=1.000000)" :!class /Script/Engine.MaterialInstanceDynamic))))

(event EventBeginPlay
  (bind _plane (Variables|Default|GetPlane))
  (bind _returnvalue (Rendering|Material|CreateDynamicMaterialInstance _plane 0 "/Game/Materials/Mat_PushBlock.Mat_PushBlock" "None" :!class /Script/Engine.PrimitiveComponent))
  (Rendering|Material|SetMaterial _plane 0 _returnvalue)
  (Rendering|Material|SetScalarParameterValue _returnvalue "Intensity" 2e+01 :!class /Script/Engine.MaterialInstanceDynamic)
  (Rendering|Material|SetVectorParameterValue _returnvalue "Color" "(R=1.000000,G=0.000000,B=0.000000,A=1.000000)" :!class /Script/Engine.MaterialInstanceDynamic))

(fn ConstructionScript)