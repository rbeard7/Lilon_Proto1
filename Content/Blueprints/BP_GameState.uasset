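; BP_GameState is a Blueprint that tracks whether the player has collected every orb in the current level.
; Each Tick it casts the player pawn to ThirdPersonCharacter and compares its OrbsCollected against the per-level maximum in OrbQuantityMaxPerLevel, indexed by CurrentLevel.
; On a match it sets that level's entry in AcquiredAllInEachLevel to true, polling rather than reacting to pickup events.
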(event EventBeginPlay)

(event EventTick
  (params (DeltaSeconds :type Float%20%28single-precision%29))
  (bind _asthird_person_character (Utilities|Casting|CastToThirdPersonCharacter (Game|GetPlayerCharacter 0)))
  (if (== (Variables|/Game/Archive/ThirdPersonBP/Blueprints/ThirdPersonCharacter.ThirdPersonCharacter_C|GetOrbsCollected _asthird_person_character) (Utilities|Array|Get(acopy) (Variables|Default|GetOrbQuantityMaxPerLevel) (- (Variables|Default|GetCurrentLevel) 1)))
    (Utilities|Array|SetArrayElem (Variables|Default|GetAcquiredAllInEachLevel) (- (Variables|Default|GetCurrentLevel) 1) true)))

(fn ConstructionScript)