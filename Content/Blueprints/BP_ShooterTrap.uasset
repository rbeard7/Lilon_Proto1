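; Shooter trap actor that kills the player character when it crosses the trap's line of fire.
; Every Tick, it runs a Visibility line trace from its static mesh 1000 units along world -X, regardless of rotation, with persistent debug drawing.
; If the hit actor is player 0's ThirdPersonCharacter, it sets that character's Alive flag to false.
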(event EventBeginPlay)

(event Collision|EventActorBeginOverlap
  (params (OtherActor :type Actor%20Object%20Reference)))

(event EventTick
  (params (DeltaSeconds :type Float%20%28single-precision%29))
  (bind _outhit (Collision|LineTraceByChannel (Transformation|GetWorldLocation (Variables|Default|GetStaticMesh)) (+ (Transformation|GetWorldLocation (Variables|Default|GetStaticMesh)) "-1000.000000, 0, 0") "TraceTypeQuery1" false 0 "Persistent"))
  (bind _asthird_person_character (Utilities|Casting|CastToThirdPersonCharacter (Game|GetPlayerCharacter 0)))
  (if (== _asthird_person_character (.HitActor (Collision|BreakHitResult _outhit)))
    (Variables|/Game/Archive/ThirdPersonBP/Blueprints/ThirdPersonCharacter.ThirdPersonCharacter_C|SetAlive? _asthird_person_character false)))

(fn ConstructionScript)