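; BP_SpikeBall is a spike ball that moves between two relative points, A and B, using an InterpToMovement component.
; The construction script builds the control points and sets the travel time from the A, B and Duration variables.
; Tick polls BP_GameState and activates the movement, without reset, while the current level's AcquiredAllInEachLevel flag is true.
; The Blueprint contains no active overlap or damage logic.
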(event EventBeginPlay)

(event Collision|EventActorBeginOverlap
  (params (OtherActor :type Actor%20Object%20Reference)))

(event EventTick
  (params (DeltaSeconds :type Float%20%28single-precision%29))
  (bind _asbp_game_state (Utilities|Casting|CastToBP_GameState (Game|GetGameState)))
  (if (Utilities|Array|Get(acopy) (Variables|/Game/Blueprints/BP_GameState.BP_GameState_C|GetAcquiredAllInEachLevel _asbp_game_state) (- (Variables|/Game/Blueprints/BP_GameState.BP_GameState_C|GetCurrentLevel _asbp_game_state) 1))
    (Components|Activation|Activate (Variables|Default|GetInterpToMovement) false)))

(fn ConstructionScript
  (bind _interptomovement (Variables|Default|GetInterpToMovement))
  (Variables|/Script/Engine.InterpToMovementComponent|SetControlPoints _interptomovement (Utilities|Array|MakeArray (Utilities|Struct|MakeInterpControlPoint (Variables|Default|GetA) true) (Utilities|Struct|MakeInterpControlPoint (Variables|Default|GetB) true)))
  (Variables|/Script/Engine.InterpToMovementComponent|SetDuration _interptomovement (Variables|Default|GetDuration)))